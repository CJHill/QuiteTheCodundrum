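; Maze actor that builds a seeded, grid-based maze in its Construction Script, placing path tiles as hierarchical instanced meshes spaced by TileSize.
; GenerateMaze picks a random start, recursively carves through valid neighbours and backtracks via ToCheck, recording dead ends in EndPaths.
; A custom DoNPlus macro limits the neighbour retries at each tile.
; Keys 2, 3 and 4 are spawning experiments, while GenerateGrid is only called from disconnected nodes.
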(event Input|KeyboardEvents|1
  (params (Key :type Key%20Structure :default "None")))

(event Input|KeyboardEvents|3
  (params (Key :type Key%20Structure :default "None"))
  (bind _defaultsceneroot (Variables|Default|GetDefaultSceneRoot))
  (bind _returnvalue (Components|GetOwner _defaultsceneroot))
  (:Pressed
    (bind _returnvalue_2 (AddComponent|AddInstancedStaticMeshComponent (Components|GetOwner (Variables|Default|GetDefaultSceneRoot)) false (Math|Transform|MakeTransform "10.000000,30.000000,5000.000000" (Transformation|GetActorRotation _returnvalue) (Transformation|GetActorScale3D _returnvalue))))
    (Development|PrintString (Utilities|String|ToString(Transform) (.OutInstanceTransform (Components|InstancedStaticMesh|GetInstanceTransform _returnvalue_2 0 false))))))

(event Input|KeyboardEvents|2
  (params (Key :type Key%20Structure :default "None"))
  (:Pressed
    (CallFunction|GenerateGridCell (Transformation|GetActorLocation))))

(event Input|KeyboardEvents|4
  (params (Key :type Key%20Structure :default "None"))
  (bind _defaultsceneroot (Variables|Default|GetDefaultSceneRoot))
  (bind _returnvalue (Components|GetOwner _defaultsceneroot))
  (:Pressed
    (bind _returnvalue_2 (Game|SpawnActorfromClass "Maze_BP_C" (Math|Transform|MakeTransform "10.000000,30.000000,5000.000000" (Transformation|GetActorRotation _returnvalue) (Transformation|GetActorScale3D _returnvalue)) "AlwaysSpawn" 0 0))
    (Development|PrintString (Utilities|String|ToString(Transform) (Transformation|GetActorTransform _returnvalue_2)) true true "(R=0.000000,G=1.000000,B=0.261168,A=1.000000)")))

(fn ConstructionScript
  (bind _pathtiles_output (CallFunction|GenerateMaze :Seed (Variables|Default|GetSeed) :InputSize (Variables|Default|GetMazeSize)))
  (bind _result (Utilities|Set|ToArray _pathtiles_output))
  (for _array_element _result
    (Components|InstancedStaticMesh|AddInstance (Variables|Default|GetHierarchicalInstancedStaticMesh) (Math|Transform|MakeTransform (Math|Vector|MakeVector (* (.X (Utilities|Struct|BreakIntPoint _array_element)) (Variables|Default|GetTileSize)) (* (.Y (Utilities|Struct|BreakIntPoint _array_element)) (Variables|Default|GetTileSize)) 0.0)) false)))

(fn GenerateGrid
  (params (Grid_Size :type Int%20Point%20Structure))
  (bind (_x _y) (Utilities|Struct|BreakIntPoint Grid_Size))
  ;[1 1 1] Code after loop from completion of first for Loop
  (for _index (range 1 _x)
    (for _index_2 (range 1 _y)
      (CallFunction|GenerateGridCell (* (Math|Vector|MakeVector (Math|Conversions|ToFloat(Integer) _index) (Math|Conversions|ToFloat(Integer) _index_2) 0.0) "300.000000,300.000000,0.000000"))))
  (Development|PrintString "Hello"))

(fn GenerateGridCell
  (params (BottomWallPos :type Vector))
  (bind _returnvalue (Transformation|GetActorTransform))
  (bind _returnvalue_2 (Transformation|GetActorTransform))
  (bind _returnvalue_3 (Transformation|GetActorTransform))
  (bind (_location _rotation _scale) (Math|Transform|BreakTransform _returnvalue))
  (bind (_location_2 _rotation_2 _scale_2) (Math|Transform|BreakTransform _returnvalue_2))
  (bind (_location_3 _rotation_3 _scale_3) (Math|Transform|BreakTransform _returnvalue_3))
  (Game|SpawnActorfromClass "Maze_BP_C" (Math|Transform|MakeTransform (+ BottomWallPos "300.000000,300.000000,0.000000") (Math|Rotator|MakeRotfromZ (+ _rotation "0.000000,0.000000,90.000000")) _scale) "Undefined" 0 0)
  (Game|SpawnActorfromClass "Maze_BP_C" (Math|Transform|MakeTransform (+ BottomWallPos "300.000000,-300.000000,0.000000") (Math|Rotator|MakeRotfromZ (+ _rotation_2 "0.000000,0.000000,90.000000")) _scale_2) "Undefined" 0 0)
  (Game|SpawnActorfromClass "Maze_BP_C" (Math|Transform|MakeTransform (+ BottomWallPos "600.000000,0.000000,0.000000") _rotation_3 _scale_3) "Undefined" 0 0))

(fn GenerateMaze
  (params (InputStream :type Random%20Stream%20Structure) (Seed :type Integer) (InputSize :type Int%20Point%20Structure))
  (Math|Random|SetRandomStreamSeed InputStream Seed)
  (LocalVariables|SetRandStream InputStream)
  (bind _output_get (LocalVariables|SetStartLoc (Utilities|GetRandLocation InputSize (LocalVariables|GetRandStream))))
  (LocalVariables|SetCurrentLoc _output_get)
  (CallFunction|AddNeighbourLocation (LocalVariables|GetSize) (LocalVariables|GetCurrentLoc) (LocalVariables|GetRandStream) (LocalVariables|GetPathTiles) (LocalVariables|GetBridgeTiles) (LocalVariables|GetToCheck) (LocalVariables|GetEndPaths) :!label _label)
  (if (> (Utilities|Set|Length (LocalVariables|GetToCheck)) 0)
    (CallFunction|Backtrack (LocalVariables|GetCurrentLoc) (LocalVariables|GetToCheck) (LocalVariables|GetBridgeTiles) (LocalVariables|GetPathTiles))
    (goto _label)
    (else
      (return (LocalVariables|GetPathTiles) (LocalVariables|GetEndPaths)))))

(fn AddNeighbourLocation
  (params (Size :type Int%20Point%20Structure) (CurrentLocation :type Int%20Point%20Structure) (RandStream :type Random%20Stream%20Structure) (PathTiles :type Set%20of%20Int%20Point%20Structures) (BridgeTiles :type Set%20of%20Int%20Point%20Structures) (ToCheck :type Set%20of%20Int%20Point%20Structures) (EndPaths :type Set%20of%20Int%20Point%20Structures))
  (LocalVariables|SetNeighbourIndex (Math|Random|RandomIntegerinRangefromStream 1 3 RandStream))
  (if (Utilities|CheckifLocationIsValid (.Floor (Utilities|GetNeighbourandBridge CurrentLocation (LocalVariables|GetNeighbourIndex))) Size PathTiles BridgeTiles) :!label _label
    (Utilities|Set|Add PathTiles (.Floor (Utilities|GetNeighbourandBridge CurrentLocation (LocalVariables|GetNeighbourIndex))))
    (Utilities|Set|Add BridgeTiles (.Floor (Utilities|GetNeighbourandBridge CurrentLocation (LocalVariables|GetNeighbourIndex))))
    (Utilities|Set|Add ToCheck (.Floor (Utilities|GetNeighbourandBridge CurrentLocation (LocalVariables|GetNeighbourIndex))))
    (CallFunction|AddNeighbourLocation Size (.Floor (Utilities|GetNeighbourandBridge CurrentLocation (LocalVariables|GetNeighbourIndex))) RandStream PathTiles BridgeTiles ToCheck EndPaths)
    (else
      (Utilities|DoNPlus 4
        (:Exit
          (LocalVariables|SetNeighbourIndex (Math|Integer|SelectInt 0 (+ (LocalVariables|GetNeighbourIndex) 1) (>= (+ (LocalVariables|GetNeighbourIndex) 1) 4)))
          (goto _label))
        (:Exceeds%20Nth
          (bind _count (CallFunction|GetNeighbourCount CurrentLocation PathTiles))
          (if (== _count 1)
            (Utilities|Set|Add EndPaths CurrentLocation)))))))

(fn GetNeighbourCount
  (params (CurrentLocation :type Int%20Point%20Structure) (PathTiles :type Set%20of%20Int%20Point%20Structures))
  (for _array_element (Utilities|GetNeighbourLocation CurrentLocation)
    (if (Utilities|Set|Contains PathTiles _array_element)
      (Math|Integer|IncrementInt (LocalVariables|GetCounter))))
  (return (LocalVariables|GetCounter)))

(fn Backtrack
  (params (CurrentTile :type Int%20Point%20Structure%20%28by%20ref%29) (ToCheck :type Set%20of%20Int%20Point%20Structures) (BridgeTiles :type Set%20of%20Int%20Point%20Structures) (PathTiles :type Set%20of%20Int%20Point%20Structures))
  (bind _result (Utilities|Set|ToArray ToCheck))
  (|SetBy-RefVar CurrentTile (Utilities|Array|Get(acopy) _result (Utilities|Array|LastIndex _result)))
  (Utilities|Array|RemoveItem _result (Utilities|Array|Get(acopy) _result (Utilities|Array|LastIndex _result)))
  (bind _result_2 (Utilities|Set|ToArray BridgeTiles))
  (Utilities|Set|Add PathTiles (Utilities|Array|Get(acopy) _result_2 (Utilities|Array|LastIndex _result_2)))
  (Utilities|Set|Remove BridgeTiles (Utilities|Array|Get(acopy) _result_2 (Utilities|Array|LastIndex _result_2))))