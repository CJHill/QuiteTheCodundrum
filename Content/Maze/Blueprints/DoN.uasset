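; DoN is a maze test actor that compares spawning actors with adding hierarchical instanced static mesh components' instances through debug keys.
; Key 4 spawns another DoN and key 3 adds a mesh instance, both at fixed coordinates with the owner's rotation and scale, printing results.
; It also defines a DoN+ macro, unused here: a resettable Do N that outputs its count and fires OverNth beyond the limit.
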(event Input|KeyboardEvents|3
  (params (Key :type Key%20Structure :default "None"))
  (bind _defaultsceneroot (Variables|Default|GetDefaultSceneRoot))
  (bind _returnvalue (Components|GetOwner _defaultsceneroot))
  (:Pressed
    (Development|PrintString "Key 3 pressed - Instanced Static Mesh")
    (bind _returnvalue_2 (Components|InstancedStaticMesh|AddInstance (Variables|Default|GetHierarchicalInstancedStaticMesh) (Math|Transform|MakeTransform "100.000000,30.000000,50.000000" (Transformation|GetActorRotation _returnvalue) (Transformation|GetActorScale3D _returnvalue)) false))
    (Development|PrintString (Utilities|String|ToString(Integer) _returnvalue_2))))

(event Input|KeyboardEvents|4
  (params (Key :type Key%20Structure :default "None"))
  (bind _defaultsceneroot (Variables|Default|GetDefaultSceneRoot))
  (bind _returnvalue (Components|GetOwner _defaultsceneroot))
  (:Pressed
    (Development|PrintString "Key 4 pressed - Spawn Actor")
    (bind _returnvalue_2 (Game|SpawnActorfromClass "DoN_C" (Math|Transform|MakeTransform "100.000000,30.000000,50.000000" (Transformation|GetActorRotation _returnvalue) (Transformation|GetActorScale3D _returnvalue)) "AlwaysSpawn" 0 0))
    (Development|PrintString (Utilities|String|ToString(Transform) (Transformation|GetActorTransform _returnvalue_2)) true true "(R=0.000000,G=1.000000,B=0.261168,A=1.000000)")))

(fn ConstructionScript)