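; Melee enemy AI character with an attack range component and a function that sets its movement component's max walk speed.
; The attack range overlap events are currently empty.
; Disconnected debug-printing logic would toggle the ReadytoAttack blackboard key and an attack animation flag, with a player character cast on the clearing branch.
; An author note ties changes in the attack sequence to the Behavior Tree.
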(event OnComponentBeginOverlap(attackrange)
  (params (OverlappedComponent :type Primitive%20Component%20Object%20Reference) (OtherActor :type Actor%20Object%20Reference) (OtherComp :type Primitive%20Component%20Object%20Reference) (OtherBodyIndex :type Integer) (bFromSweep :type Boolean) (SweepResult :type Hit%20Result%20Structure%20%28by%20ref%29)))

(event OnComponentEndOverlap(attackrange)
  (params (OverlappedComponent :type Primitive%20Component%20Object%20Reference) (OtherActor :type Actor%20Object%20Reference) (OtherComp :type Primitive%20Component%20Object%20Reference) (OtherBodyIndex :type Integer))
  ;[1 1 1] If attack sequnce needs to be changed disconnect this node and in the BT connect the task set attack bool to false to the sequence and add a wait
)

(event EventBeginPlay)

(event Collision|EventActorBeginOverlap
  (params (OtherActor :type Actor%20Object%20Reference)))

(fn ConstructionScript)

(fn UpdateWalkSpeed
  (params (NewWalkSpeed :type Float%20%28double-precision%29))
  (Variables|/Script/Engine.CharacterMovementComponent|SetMaxWalkSpeed (Variables|Character|GetCharacterMovement) NewWalkSpeed))