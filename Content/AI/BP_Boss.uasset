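; BP_Boss is a boss enemy character that feeds its state to an AI Blackboard.
; BeginPlay and Tick write Health to the Blackboard, and Tick also sets HasLowHealth for an intended sub-40% attack mode.
; That check compares Health against 40% of itself, so positive health never counts as low.
; UpdateWalkSpeed sets movement speed, while melee, ranged and too-close flag logic, including attack animation flags, is disconnected and never runs.
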(event EventBeginPlay
  ;[1 1 1] It may be better to keep the health value in the BP but in case it is needed in the black board
  (AI|Components|Blackboard|SetValueasFloat (AI|GetBlackboard 0) (Utilities|Name|MakeLiteralName "Health") (Variables|Default|GetHealth)))

(event Collision|EventActorBeginOverlap
  (params (OtherActor :type Actor%20Object%20Reference)))

(event EventTick
  (params (DeltaSeconds :type Float%20%28single-precision%29))
  (AI|Components|Blackboard|SetValueasFloat (AI|GetBlackboard 0) (Utilities|Name|MakeLiteralName "Health") (Variables|Default|GetHealth))
  ;[1 1 1] Sets the bool responsible for the elite enemy attack mode
  (if (<= (Variables|Default|GetHealth) (* (Variables|Default|GetHealth) 0.4))
    (AI|Components|Blackboard|SetValueasBool (AI|GetBlackboard 0) (Utilities|Name|MakeLiteralName "HasLowHealth") true)
    (else
      (AI|Components|Blackboard|SetValueasBool (AI|GetBlackboard 0) (Utilities|Name|MakeLiteralName "HasLowHealth") false))))

(fn ConstructionScript)

(fn UpdateWalkSpeed
  (params (NewWalkSpeed :type Float%20%28double-precision%29))
  (Variables|/Script/Engine.CharacterMovementComponent|SetMaxWalkSpeed (Variables|Character|GetCharacterMovement) NewWalkSpeed))